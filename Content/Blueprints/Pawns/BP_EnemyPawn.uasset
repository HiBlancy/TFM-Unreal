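; BP_EnemyPawn is an enemy pawn that displays its health on a widget bar.
; Every tick it copies the Health component's percentage into the WBP_EnemyHealth progress bar.
; It then rotates the bar with a look-at from its world location, using the player camera's forward vector as the target point rather than the camera's position.
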(event `self.ReceiveTick`
  (params (DeltaSeconds :type "Float (single-precision)"))
  (bind _healthbar (`self.HealthBar`))
  ;[1 1 1] Barra de vida del enemigo
  (bind _aswbp_enemy_health (cast `/Game/Blueprints/Widgets/WBP_EnemyHealth` (`WidgetComponent.GetWidget` (`self.HealthBar`))))
  (`ProgressBar.SetPercent` (`/Game/Blueprints/Widgets/WBP_EnemyHealth.ProgressBar_0` _aswbp_enemy_health) (`HealthComponent.GetHealthPercent` (`self.Health`)))
  (`SceneComponent.K2_SetWorldRotation` _healthbar (`KismetMathLibrary.FindLookAtRotation` (`SceneComponent.K2_GetComponentLocation` _healthbar) (`KismetMathLibrary.Conv_RotatorToVector` (`SceneComponent.K2_GetComponentRotation` (`PlayerCameraManager.TransformComponent` (`GameplayStatics.GetPlayerCameraManager` 0))))) false false))

(fn `UserConstructionScript`)