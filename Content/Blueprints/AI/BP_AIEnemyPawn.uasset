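; AI enemy pawn Blueprint that keeps its on-screen health bar widget updated.
; Each Tick casts the EnemyHealth component's widget to WBP_EnemyHealth and sets its progress bar from the Health component's percentage.
; It then rotates the widget using a look-at from its location toward the player camera's forward vector, which serves as the target point instead of the camera's position.
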(event `self.ReceiveTick`
  (params (DeltaSeconds :type "Float (single-precision)"))
  (bind _enemyhealth (`self.EnemyHealth`))
  ;[1 1 1] Health widget on screen
  (bind _aswbp_enemy_health (cast `/Game/Blueprints/Widgets/WBP_EnemyHealth` (`WidgetComponent.GetWidget` (`self.EnemyHealth`))))
  (`ProgressBar.SetPercent` (`/Game/Blueprints/Widgets/WBP_EnemyHealth.ProgressBar_0` _aswbp_enemy_health) (`HealthComponent.GetHealthPercent` (`self.Health`)))
  (`SceneComponent.K2_SetWorldRotation` _enemyhealth (`KismetMathLibrary.FindLookAtRotation` (`SceneComponent.K2_GetComponentLocation` _enemyhealth) (`KismetMathLibrary.Conv_RotatorToVector` (`SceneComponent.K2_GetComponentRotation` (`PlayerCameraManager.TransformComponent` (`GameplayStatics.GetPlayerCameraManager` 0))))) false false))

(fn `UserConstructionScript`)